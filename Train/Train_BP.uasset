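; Train actor that departs along a spline path when the third-person character enters its trigger, playing only while it has not already started travelling.
; On departure it raises the audio volume and plays the Start timeline, whose value sets the speed.
; A short Delay loop advances distance by speed until the end of the ActivePath spline.
; MoveAlong places the root at that distance, following only the spline's yaw.
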(event OnComponentBeginOverlap(Trigger)
  (params (OverlappedComponent :type Primitive%20Component%20Object%20Reference) (OtherActor :type Actor%20Object%20Reference) (OtherComp :type Primitive%20Component%20Object%20Reference) (OtherBodyIndex :type Integer) (bFromSweep :type Boolean) (SweepResult :type Hit%20Result%20Structure%20%28by%20ref%29))
  (bind _activepath (Variables|Default|GetActivePath))
  (bind _spline (Variables|/Game/Train/Path.Path_C|GetSpline _activepath))
  (Utilities|Casting|CastToBP_ThirdPersonCharacter OtherActor)
  (if (not (Variables|Default|GetTravel))
    (Audio|Components|Audio|SetVolumeMultiplier (Variables|Default|GetAudio) 1.0 :!class /Script/Engine.AudioComponent)
    (bind _start (Timeline|Start PlayFromStart)
      (:Update
        (Variables|Default|SetSpeed _start)
        (Variables|Default|SetTravel true)
        (if (< (Variables|Default|GetDistance) (Spline|GetSplineLength _spline)) :!label _label
          (CallFunction|MoveAlong _spline (Variables|Default|GetDistance))
          (Variables|Default|SetDistance (+ (Variables|Default|GetDistance) (Variables|Default|GetSpeed)))
          (Utilities|FlowControl|Delay 0.001)
          (goto _label))))))

(fn ConstructionScript)

(fn MoveAlong
  (params (Path :type Spline%20Component%20Object%20Reference) (Distance :type Float%20%28double-precision%29))
  (bind _defaultsceneroot (Variables|Default|GetDefaultSceneRoot))
  (Transformation|SetWorldLocation _defaultsceneroot (Spline|GetLocationatDistanceAlongSpline Path Distance "World") false false)
  (Transformation|SetWorldRotation _defaultsceneroot (Math|Rotator|MakeRotator 0.0 0.0 (.yaw (Spline|GetRotationatDistanceAlongSpline Path Distance "Local"))) false false))