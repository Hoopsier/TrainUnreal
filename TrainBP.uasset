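; Train actor that rides along splines, spinning its wheels, sliding paired doors and showing speed on a speedometer.
; Start and stop timelines set Speed, while a RetriggerableDelay loop advances Distance along Path.
; At a spline's end it hands off to the next PathSpline or SplitPath.
; It starts on BeginPlay or when the player enters its trigger while idle, and restarts after a stop if the player remains inside.
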(event OnComponentBeginOverlap(Trigger)
  (params (OverlappedComponent :type Primitive%20Component%20Object%20Reference) (OtherActor :type Actor%20Object%20Reference) (OtherComp :type Primitive%20Component%20Object%20Reference) (OtherBodyIndex :type Integer) (bFromSweep :type Boolean) (SweepResult :type Hit%20Result%20Structure%20%28by%20ref%29))
  (bind _asbp_third_person_character (Utilities|Casting|CastToBP_ThirdPersonCharacter OtherActor))
  (Variables|Default|SetOver true)
  (if (not (Variables|Default|GetTraveling))
    (if (== _asbp_third_person_character (Variables|Default|GetPlayer))
      _
      (else
        (Variables|Default|SetPlayer _asbp_third_person_character)))
    (CallFunction|StartEvent)))

(event OnComponentEndOverlap(Trigger)
  (params (OverlappedComponent :type Primitive%20Component%20Object%20Reference) (OtherActor :type Actor%20Object%20Reference) (OtherComp :type Primitive%20Component%20Object%20Reference) (OtherBodyIndex :type Integer))
  (Utilities|Casting|CastToBP_ThirdPersonCharacter OtherActor)
  (Variables|Default|SetOver false))

(event Custom|Stop
  (Variables|Default|SetStopping true)
  (bind _start (Timeline|StopTL PlayFromStart)
    (:Update
      (Variables|Default|SetSpeed _start))
    (:Finished
      (Audio|Components|Audio|SetVolumeMultiplier (Variables|Default|GetAudio) 0.0 :!class /Script/Engine.AudioComponent)
      (CallFunction|OpenCloseDoors false)
      (Utilities|FlowControl|Delay 3.0)
      (if (Variables|Default|GetOver)
        (CallFunction|StartEvent)
        (Development|PrintString "True")
        (else
          (Variables|Default|SetTraveling false)
          (Development|PrintString "False"))))))

(event Custom|StartEvent
  (bind _nextspline (Variables|Default|GetNextSpline))
  (bind _path (Variables|Default|GetPath))
  (bind _returnvalue (Components|GetOwner _nextspline))
  (CallFunction|OpenCloseDoors true)
  (Variables|Default|SetStopping false)
  (Utilities|FlowControl|Delay 1.0)
  (Audio|Components|Audio|SetVolumeMultiplier (Variables|Default|GetAudio) 1.0 :!class /Script/Engine.AudioComponent)
  (bind _start (Timeline|Start PlayFromStart)
    (:Update
      (if (not (Variables|Default|GetStopping))
        (Variables|Default|SetSpeed _start)
        (Variables|Default|SetTraveling true)
        (if (< (Variables|Default|GetDistance) (Spline|GetSplineLength _path)) :!label _label
          (CallFunction|MoveAlong _path (Variables|Default|GetDistance))
          (Variables|Default|SetDistance (+ (Variables|Default|GetSpeed) (Variables|Default|GetDistance)))
          (CallFunction|WheelSpin)
          (Utilities|FlowControl|RetriggerableDelay 0.001)
          (goto _label)
          (else
            (Variables|Default|SetDistance 0.0)
            (if (Utilities|IsValid _returnvalue) ; This one can clear up an unknown reason of error or train stopping
              (bind _aspath_spline (Utilities|Casting|CastToPathSpline _returnvalue)
                (:then
                  (Default|UseThis _aspath_spline)
                  (Utilities|FlowControl|DelayUntilNextTick)
                  (Default|Initialize _aspath_spline)
                  (goto _label))
                (:CastFailed
                  (bind _assplit_path (Utilities|Casting|CastToSplitPath _returnvalue))
                  (Default|UseThis _assplit_path)
                  (Utilities|FlowControl|DelayUntilNextTick)
                  (Default|Initialize _assplit_path)
                  (goto _label))))))))))

(event Custom|WheelSpin
  ;[1 0 0] Wheel spin
  (for _array_element (Variables|Default|GetWheels)
    (Transformation|AddLocalRotation _array_element (Math|Rotator|MakeRotator 0.0 0.0 (* (Variables|Default|GetSpeed) -1.0)) false false)))

(event Custom|OpenCloseDoors
  (params (Open :type Boolean))
  (bind _doorspeed (Variables|Default|GetDoorSpeed))
  (bind _doorspeed_2 (Variables|Default|GetDoorSpeed))
  (bind _returnvalue (* _doorspeed -1.0))
  ;[0 0.6148 1] Doors
  (Timeline|Doors PlayFromStart
    (:Update
      (if Open
        (if (> (Variables|Default|GetDoorDistance) (Variables|Default|GetDoorMaxDist))
          (Timeline|Doors Stop)
          (else
            (Variables|Default|SetDoorDistance (+ _doorspeed_2 (Variables|Default|GetDoorDistance)))
            (for (_array_element _array_index) (Variables|Default|GetLeftDoors) :!label _label
              (if Open
                (CallFunction|MoveDoors _returnvalue _array_element false)
                (CallFunction|MoveDoors _returnvalue (Utilities|Array|Get(acopy) (Variables|Default|GetRightDoors) _array_index) true)
                (else
                  (CallFunction|MoveDoors _doorspeed _array_element false)
                  (CallFunction|MoveDoors _doorspeed (Utilities|Array|Get(acopy) (Variables|Default|GetRightDoors) _array_index) true))))))
        (elif (< (Variables|Default|GetDoorDistance) 0.0)
          (Timeline|Doors Stop)
          (else
            (Variables|Default|SetDoorDistance (- (Variables|Default|GetDoorDistance) _doorspeed_2))
            (goto _label)))))))

(event EventBeginPlay
  (bind _leftdoors (Variables|Default|GetLeftDoors))
  (bind _rightdoors (Variables|Default|GetRightDoors))
  (bind _wheels (Variables|Default|GetWheels))
  ;[0 0.6148 1] Doors
  (Utilities|Array|Add _leftdoors (Variables|Default|GetLDoor))
  (Utilities|Array|Add _leftdoors (Variables|Default|GetLDoor1))
  (Utilities|Array|Add _leftdoors (Variables|Default|GetLDoor2))
  (Utilities|Array|Add _leftdoors (Variables|Default|GetLDoor3))
  (Utilities|Array|Add _rightdoors (Variables|Default|GetRDoor))
  (Utilities|Array|Add _rightdoors (Variables|Default|GetRDoor1))
  (Utilities|Array|Add _rightdoors (Variables|Default|GetRDoor2))
  (Utilities|Array|Add _rightdoors (Variables|Default|GetRDoor3))
  (Utilities|Array|Add _wheels (Variables|Default|GetWheel))
  (Utilities|Array|Add _wheels (Variables|Default|GetWheel1))
  (Utilities|Array|Add _wheels (Variables|Default|GetWheel2))
  (Utilities|Array|Add _wheels (Variables|Default|GetWheel3))
  (Utilities|Array|Add _wheels (Variables|Default|GetWheel4))
  (Utilities|Array|Add _wheels (Variables|Default|GetWheel5))
  (CallFunction|StartEvent))

(fn ConstructionScript)

(fn MoveAlong
  (params (Path :type Spline%20Component%20Object%20Reference) (Distance :type Float%20%28double-precision%29))
  (bind _returnvalue (Spline|GetRotationatDistanceAlongSpline Path Distance "Local"))
  (bind _defaultsceneroot (Variables|Default|GetDefaultSceneRoot))
  (Transformation|SetWorldLocation _defaultsceneroot (Spline|GetLocationatDistanceAlongSpline Path Distance "World") false false)
  (Transformation|SetWorldRotation _defaultsceneroot (Math|Rotator|MakeRotator 0.0 (.pitch _returnvalue) (+ (.yaw _returnvalue) 9e+01)) false false)
  (Rendering|Components|TextRender|SetText (Variables|Default|GetSpeedometer) (Utilities|Text|ToText(Float) (Variables|Default|GetSpeed) "HalfToEven" false true 1 324 0 0)))

(fn MoveDoors
  (params (Speed :type Float%20%28double-precision%29) (Door :type Scene%20Component%20Object%20Reference) (Right :type Boolean))
  (bind _relativelocation (Variables|/Script/Engine.SceneComponent|GetRelativeLocation Door))
  (if Right
    (Transformation|SetRelativeLocation Door (Math|Vector|MakeVector (.x _relativelocation) (+ Speed (.y _relativelocation)) (.z _relativelocation)) false false)
    (else
      (Transformation|SetRelativeLocation Door (Math|Vector|MakeVector (.x _relativelocation) (- (.y _relativelocation) Speed) (.z _relativelocation)) false false))))